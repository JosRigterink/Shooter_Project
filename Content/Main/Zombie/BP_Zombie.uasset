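; BP_Zombie is a zombie enemy that chases and attacks the player.
; From BeginPlay it runs an AI MoveTo targeting player controller 0, retrying on failure and playing an attack montage on success.
; When the montage completes it resumes the chase, forming a move-attack loop with no damage logic in this graph.
; PawnSensing only raises the walk speed when it sees a pawn, and nothing here lowers it again.
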(event `self.PawnSensing.OnSeePawn`
  (params (Pawn :type "Pawn Object Reference"))
  (set `CharacterMovementComponent.MaxWalkSpeed` 360.0 (`self.CharacterMovement`)))

(event `self.ReceiveBeginPlay`
  (`self.RunToPlayer`))

(event `RunToPlayer`
  (`|AIMoveTo` self (0.0 0.0 0.0) (`GameplayStatics.GetPlayerController` 0) 40.0
    (:`OnSuccess`
      (`self.AttackPlayer`))
    (:`OnFail`
      (`self.RunToPlayer`))))

(event `AttackPlayer`
  (`|PlayMontage` (`self.Mesh`) "/Game/Main/Zombie/Animations/zombie_attack_Montage1.zombie_attack_Montage1"
    (:`OnCompleted`
      (`self.RunToPlayer`))))

(fn `UserConstructionScript`)